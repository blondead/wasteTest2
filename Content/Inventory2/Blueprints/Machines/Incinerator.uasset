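; Interactable incinerator machine that opens item slots beside the player's inventory and computes pollution and energy from their contents.
; On first interact it spawns and caches an IncineratorsBP container, then shows both UIs, with a DoOnce gate reset on close.
; Incinerate adds quantity-scaled pollution by the item's Incinerate flag, halved with an air purifier, while Energy totals yield from flagged items.
; Both loops return on the first slot, and Incinerate always reports failure.
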(event `OnInteract`
  (params (FirstPersonCharacter :type "/Game/FirstPersonBP/Blueprints/FirstPersonCharacter Object Reference"))
  (bind _incineratorref (`self.IncineratorRef`))
  (bind _inventoryref (`/Game/FirstPersonBP/Blueprints/FirstPersonCharacter.InventoryRef` (`self.FirstPersonCharacter`)))
  (bind _button_1926 (`/Game/Inventory2/Widget/InventoryWidgt.Button_1926` (`/Game/Inventory2/Blueprints/InventoryBP.Inventory Widgt` _inventoryref)))
  (bind _output_get (set `self.Terminal` true))
  (`/Engine/EditorBlueprintResources/StandardMacros.DoOnce` false :!label _label
    (:`Completed`
      (set `self.FirstPersonCharacter` FirstPersonCharacter)
      (`/Engine/EditorBlueprintResources/StandardMacros.IsValid` (`self.IncineratorRef`)
        (:`Is Valid`
          _)
        (:`Is Not Valid`
          (bind _returnvalue (`|SpawnActorFromClass` "/Game/Inventory2/Blueprints/IncineratorsBP.IncineratorsBP_C" (`KismetMathLibrary.MakeTransform` (0.0 0.0 0.0)) "AlwaysSpawn" "OverrideRootScale" null (`self.NoOfSlots`) (`self.FirstPersonCharacter`) (`self.SlotsPerRow`) self null))
          (set `self.IncineratorRef` _returnvalue)))
      (`/Game/Inventory2/Widget/Recycles/IncineratorWidget.GnenerateSlots` (`/Game/Inventory2/Blueprints/IncineratorsBP.Incinerator Widget 0` _incineratorref) _incineratorref)
      (`/Game/Inventory2/Blueprints/IncineratorsBP.ShowIncinerator` _incineratorref)
      (`/Game/Inventory2/Blueprints/InventoryBP.ShowInventory` _inventoryref _output_get)
      (`Widget.SetIsEnabled` _button_1926 false)
      (`Widget.SetVisibility` _button_1926 "Hidden"))))

(event `OnStorageClosed`
  (bind _inventoryref (`/Game/FirstPersonBP/Blueprints/FirstPersonCharacter.InventoryRef` (`self.FirstPersonCharacter`)))
  (bind _button_1926 (`/Game/Inventory2/Widget/InventoryWidgt.Button_1926` (`/Game/Inventory2/Blueprints/InventoryBP.Inventory Widgt` _inventoryref)))
  (set `self.Terminal` false)
  (`/Game/Inventory2/Blueprints/IncineratorsBP.HideIncinerator` (`self.IncineratorRef`))
  (`/Game/Inventory2/Blueprints/InventoryBP.HideInventory` _inventoryref (stale `OnInteract` _output_get))
  (`Widget.SetIsEnabled` _button_1926 true)
  (`Widget.SetVisibility` _button_1926 "Visible")
  (goto _label :!via `Reset`))

(fn `Energy`
  (returns (Success :type Boolean) (Energy :type Integer))
  (for _index (range (+ (`KismetArrayLibrary.Array_LastIndex` (`/Game/Inventory2/Blueprints/IncineratorsBP.Slots` (`self.IncineratorRef`))) 1))
    (bind (_empty_ _iteminfo _itemquantity) (`/Game/Inventory2/Blueprints/IncineratorsBP.GetItemInfoAtIndex` (`self.IncineratorRef`) _index))
    (if _empty_
      _
      (elif (`.Incinerate?_12_B97CCBC34B3FE71173A0888A77A15CC9` (break `/Game/Inventory2/Blueprints/Structures/ItemInfo` _iteminfo))
        (bind _output_get (set `self.TotalEnergy` (+ (* (`self.EnergyValue`) _itemquantity) (`self.TotalEnergy`))))
        (return true _output_get)
        (else
          _)))
    (return false (`self.TotalEnergy`))))

(fn `Incinerate`
  (params (`AirPurifier?` :type Boolean))
  (returns (Success :type Boolean) (Pollution :type Integer) (Index :type Integer) (Quantity :type Integer))
  (for _index (range (+ (`KismetArrayLibrary.Array_LastIndex` (`/Game/Inventory2/Blueprints/IncineratorsBP.Slots` (`self.IncineratorRef`))) 1))
    (bind (_empty_ _iteminfo _itemquantity) (`/Game/Inventory2/Blueprints/IncineratorsBP.GetItemInfoAtIndex` (`self.IncineratorRef`) _index))
    (if _empty_
      (return false (`self.Pollution`) 0 0)
      (else
        (if (`.Incinerate?_12_B97CCBC34B3FE71173A0888A77A15CC9` (break `/Game/Inventory2/Blueprints/Structures/ItemInfo` _iteminfo))
          (bind _output_get (set `self.GoodPollution` (* _itemquantity (`self.GoodPol`))))
          (set `self.Pollution` (+ (`self.Pollution`) _output_get))
          (else
            (bind _output_get_2 (set `self.BadPollution` (* _itemquantity (`self.BadPol`))))
            (set `self.Pollution` (+ (`self.Pollution`) _output_get_2))))
        (if `AirPurifier?`
          (bind _output_get_3 (set `self.Pollution` (/ (`self.Pollution`) 2)))
          (return false _output_get_3 0 0)
          (else
            (return false (`self.Pollution`) _index _itemquantity)))))))

(fn `UserConstructionScript`)