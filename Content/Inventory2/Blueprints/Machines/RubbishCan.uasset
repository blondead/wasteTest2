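; RubbishCan is an interactable machine that hands rubbish to the player's inventory a single time.
; On interact, a DoOnce gates a loop on SlotSpace that adds stacks of randomly chosen Herb or Stone through the character's InventoryRef.
; It then prints a confirmation plus the inventory's recycle and incinerate counts.
; CollectRubbish is an empty stub and PlayerInventory is unused.
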(event `OnInteract`
  (params (`First Person Character` :type "/Game/FirstPersonBP/Blueprints/FirstPersonCharacter Object Reference"))
  (bind _inventoryref (`/Game/FirstPersonBP/Blueprints/FirstPersonCharacter.InventoryRef` `First Person Character`))
  (`/Engine/EditorBlueprintResources/StandardMacros.DoOnce` false
    (:`Completed`
      (while (< (`self.SlotSpace`) 5)
        (`/Game/Inventory2/Blueprints/InventoryBP.AddItem` _inventoryref (select `int` (`KismetMathLibrary.RandomInteger` 2) :`0` "/Game/Inventory2/Blueprints/ItemClasses/Herb.Herb_C" :`1` "/Game/Inventory2/Blueprints/ItemClasses/Stone.Stone_C" :!type "/Game/Inventory2/Blueprints/ItemClasses/ItemBP Class Reference") 20)
        (bind _result (`/Engine/EditorBlueprintResources/StandardMacros.IncrementInt` (`self.SlotSpace`))
          (:`  `
            (set `self.SlotSpace` _result))))
      (`KismetSystemLibrary.PrintString` "Rubbish Collected!")
      (bind (_recycleno _incinerateno) (`/Game/Inventory2/Blueprints/InventoryBP.GetInventoryContents` _inventoryref false))
      (`KismetSystemLibrary.PrintString` (`KismetStringLibrary.Conv_IntToString` _recycleno))
      (`KismetSystemLibrary.PrintString` (`KismetStringLibrary.Conv_IntToString` _incinerateno)))))

(fn `CollectRubbish`)

(fn `UserConstructionScript`)