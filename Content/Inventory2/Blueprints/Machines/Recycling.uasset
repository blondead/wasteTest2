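; Recycling machine actor that opens a recycle storage beside the player's inventory on interact.
; It lazily spawns a RecycleBP to hold slots and UI; a DoOnce guards reopening until storage closes, and an inventory button is hidden meanwhile.
; Box overlaps set the player's NearMachine to this actor, on exit as well as entry.
; Condition empties every filled slot, lowering machine condition once for each non-recyclable one.
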(event `OnInteract`
  (params (FirstPersonCharacter :type "/Game/FirstPersonBP/Blueprints/FirstPersonCharacter Object Reference"))
  (bind _machineref (`self.MachineRef`))
  (bind _inventoryref (`/Game/FirstPersonBP/Blueprints/FirstPersonCharacter.InventoryRef` (`self.FirstPersonCharacter`)))
  (bind _button_1926 (`/Game/Inventory2/Widget/InventoryWidgt.Button_1926` (`/Game/Inventory2/Blueprints/InventoryBP.Inventory Widgt` _inventoryref)))
  (`/Engine/EditorBlueprintResources/StandardMacros.DoOnce` false :!label _label
    (:`Completed`
      (set `self.FirstPersonCharacter` FirstPersonCharacter)
      (`/Engine/EditorBlueprintResources/StandardMacros.IsValid` (`self.MachineRef`)
        (:`Is Valid`
          _)
        (:`Is Not Valid`
          (bind _returnvalue (`|SpawnActorFromClass` "/Game/Inventory2/Blueprints/RecycleBP.RecycleBP_C" (`KismetMathLibrary.MakeTransform` (0.0 0.0 0.0)) "AlwaysSpawn" "OverrideRootScale" null (`self.NoOfSlots`) (`self.FirstPersonCharacter`) (`self.SlotsPerRow`) self null))
          (set `self.MachineRef` _returnvalue)))
      (`/Game/Inventory2/Widget/Recycles/RecycleWidget.GnenerateSlots` (`/Game/Inventory2/Blueprints/RecycleBP.MachineWidget` _machineref) _machineref)
      (`/Game/Inventory2/Blueprints/RecycleBP.ShowStorage` _machineref)
      (`/Game/Inventory2/Blueprints/InventoryBP.ShowInventory` _inventoryref)
      (`Widget.SetIsEnabled` _button_1926 false)
      (`Widget.SetVisibility` _button_1926 "Hidden"))))

(event `OnStorageClosed`
  (bind _inventoryref (`/Game/FirstPersonBP/Blueprints/FirstPersonCharacter.InventoryRef` (`self.FirstPersonCharacter`)))
  (bind _button_1926 (`/Game/Inventory2/Widget/InventoryWidgt.Button_1926` (`/Game/Inventory2/Blueprints/InventoryBP.Inventory Widgt` _inventoryref)))
  (`/Game/Inventory2/Blueprints/RecycleBP.HideStorage` (`self.MachineRef`))
  (`/Game/Inventory2/Blueprints/InventoryBP.HideInventory` _inventoryref)
  (`Widget.SetIsEnabled` _button_1926 true)
  (`Widget.SetVisibility` _button_1926 "Visible")
  (goto _label :!via `Reset`))

(event `self.Box.OnComponentBeginOverlap`
  (params (OverlappedComponent :type "PrimitiveComponent Object Reference") (OtherActor :type "Actor Object Reference") (OtherComp :type "PrimitiveComponent Object Reference") (OtherBodyIndex :type Integer) (bFromSweep :type Boolean) (SweepResult :type "HitResult Structure (by ref)"))
  (bind _asfirst_person_character (cast `/Game/FirstPersonBP/Blueprints/FirstPersonCharacter` OtherActor))
  (set `/Game/FirstPersonBP/Blueprints/FirstPersonCharacter.NearMachine` self _asfirst_person_character))

(event `self.Box.OnComponentEndOverlap`
  (params (OverlappedComponent :type "PrimitiveComponent Object Reference") (OtherActor :type "Actor Object Reference") (OtherComp :type "PrimitiveComponent Object Reference") (OtherBodyIndex :type Integer))
  (bind _asfirst_person_character (cast `/Game/FirstPersonBP/Blueprints/FirstPersonCharacter` OtherActor))
  (set `/Game/FirstPersonBP/Blueprints/FirstPersonCharacter.NearMachine` self _asfirst_person_character))

(fn `Condition`
  (for _index (range (+ (`KismetArrayLibrary.Array_LastIndex` (`/Game/Inventory2/Blueprints/RecycleBP.Slots` (`self.MachineRef`))) 1))
    (bind (_empty_ _iteminfo _itemquantity) (`/Game/Inventory2/Blueprints/RecycleBP.GetItemInfoAtIndex` (`self.MachineRef`) _index))
    (if (not _empty_)
      (if (not (`.Recyclable?_10_C5C2958C440FEE08884D79A42F113F38` (break `/Game/Inventory2/Blueprints/Structures/ItemInfo` _iteminfo)))
        (bind _output_get (set `self.CurrentCondition` (- (`self.CurrentCondition`) 1)))
        (`KismetSystemLibrary.PrintString` (`KismetStringLibrary.Conv_IntToString` _output_get)))
      (`/Game/Inventory2/Blueprints/RecycleBP.RemoveItemAtIndex` (`self.MachineRef`) _index _itemquantity))))

(fn `UserConstructionScript`)