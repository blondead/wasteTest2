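; Pickup is a world item actor that adds itself to the player's inventory when touched.
; On sphere overlap with a FirstPersonCharacter, it passes its item class and quantity to that character's inventory AddItem.
; After a successful add, it keeps any leftover as its new quantity, or destroys itself when nothing remains.
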(event `self.Sphere.OnComponentBeginOverlap`
  (params (OverlappedComponent :type "PrimitiveComponent Object Reference") (OtherActor :type "Actor Object Reference") (OtherComp :type "PrimitiveComponent Object Reference") (OtherBodyIndex :type Integer) (bFromSweep :type Boolean) (SweepResult :type "HitResult Structure (by ref)"))
  (bind _asfirst_person_character (cast `/Game/FirstPersonBP/Blueprints/FirstPersonCharacter` OtherActor))
  (bind _inventoryref (`/Game/FirstPersonBP/Blueprints/FirstPersonCharacter.InventoryRef` _asfirst_person_character))
  (`/Engine/EditorBlueprintResources/StandardMacros.IsValid` _inventoryref
    (:`Is Valid`
      (bind (_success _rest) (`/Game/Inventory2/Blueprints/InventoryBP.AddItem` _inventoryref (`self.Item Class`) (`self.Quantity`)))
      (if _success
        (if (> _rest 0)
          (set `self.Quantity` _rest)
          (else
            (`self.K2_DestroyActor`)))))))

(fn `UserConstructionScript`)