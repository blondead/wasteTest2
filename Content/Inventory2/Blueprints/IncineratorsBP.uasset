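; Incinerator Blueprint that acts as a slot-based item container with its own UI widget, with no burning logic in these graphs.
; Slot functions add, remove, swap, merge and split stacks up to MaxStack, with AddItem recursing to spread overflow across slots.
; InventoryToMachine moves items in from a player inventory, and most slot edits refresh the matching widget slot.
; Show and Hide functions toggle the widget, open flag, input mode and cursor.
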(event `self.ReceiveBeginPlay`
  (set `self.Incinerator Widget 0` (`/Game/Inventory2/Widget/MainWidget.IncineratorWidget_0` (`/Game/Inventory2/Blueprints/InventoryBP.MainWidget` (`/Game/FirstPersonBP/Blueprints/FirstPersonCharacter.InventoryRef` (`self.FirstPersonCharacter`)))))
  (`KismetArrayLibrary.Array_Resize` (`self.Slots`) (`self.SlotNo`)))

(event `UpdateSlotAtIndex`
  (params (Index :type Integer))
  (`/Game/Inventory2/Widget/Recycles/IncineratorSlot.Update slot` (`|GetArrayItem` (`/Game/Inventory2/Widget/Recycles/IncineratorWidget.SlotWidget` (`self.Incinerator Widget 0`)) Index)))

(fn `AddItem`
  (params (ItemClass :type "/Game/Inventory2/Blueprints/ItemClasses/ItemBP Class Reference") (Quantity :type Integer))
  (returns (Success :type Boolean) (Rest :type Integer))
  (locals (LocalClass :type "/Game/Inventory2/Blueprints/ItemClasses/ItemBP Class Reference") (LocalQuantity :type Integer) (FoundIndex :type Integer))
  (set `local.LocalClass` ItemClass)
  (set `local.LocalQuantity` Quantity)
  (if (`.Stackable_19_F0362273495ED642AAD4648101CE2EDC` (break `/Game/Inventory2/Blueprints/Structures/ItemInfo` (defaults `Object` ItemClass)))
    (bind (_success _index) (`self.SearchAvailStack` (`local.LocalClass`)))
    (if _success
      (bind _output_get (set `local.FoundIndex` _index))
      (bind _returnvalue (+ (`.Quantity_5_98A095BD43ACF0309D55108942BDFC60` (break `/Game/Inventory2/Blueprints/Structures/InventorySlot` (`|GetArrayItem` (`self.Slots`) _output_get))) (`local.LocalQuantity`)))
      (if (> _returnvalue (`self.MaxStack`))
        (set `local.LocalQuantity` (- _returnvalue (`self.MaxStack`)))
        (`KismetArrayLibrary.Array_Set` (`self.Slots`) (`local.FoundIndex`) (make `/Game/Inventory2/Blueprints/Structures/InventorySlot` (`local.LocalClass`) (`self.MaxStack`)))
        (`self.UpdateSlotAtIndex` (`local.FoundIndex`))
        (bind (_success_2 _rest) (`self.AddItem` (`local.LocalClass`) (`local.LocalQuantity`)))
        (return true _rest)
        (else
          (`KismetArrayLibrary.Array_Set` (`self.Slots`) (`local.FoundIndex`) (make `/Game/Inventory2/Blueprints/Structures/InventorySlot` (`local.LocalClass`) _returnvalue))
          (`self.UpdateSlotAtIndex` (`local.FoundIndex`))
          (return true 0)))
      (else
        (bind (_success_3 _index_2) (`self.SearchEmptySlot`))
        (if _success_3
          (bind _output_get_2 (set `local.FoundIndex` _index_2))
          (if (> (`local.LocalQuantity`) (`self.MaxStack`))
            (`KismetArrayLibrary.Array_Set` (`self.Slots`) _output_get_2 (make `/Game/Inventory2/Blueprints/Structures/InventorySlot` (`local.LocalClass`) (`self.MaxStack`)))
            (`self.UpdateSlotAtIndex` (`local.FoundIndex`))
            (bind (_success_4 _rest_2) (`self.AddItem` (`local.LocalClass`) (- (`local.LocalQuantity`) (`self.MaxStack`))))
            (return true _rest_2)
            (else
              (`KismetArrayLibrary.Array_Set` (`self.Slots`) (`local.FoundIndex`) (make `/Game/Inventory2/Blueprints/Structures/InventorySlot` (`local.LocalClass`) (`local.LocalQuantity`)))
              (`self.UpdateSlotAtIndex` (`local.FoundIndex`))
              (return true 0)))
          (else
            (return false (`local.LocalQuantity`))))))
    (else
      (bind (_success_5 _index_3) (`self.SearchEmptySlot`))
      (if _success_5
        (bind _output_get_3 (set `local.FoundIndex` _index_3))
        (`KismetArrayLibrary.Array_Set` (`self.Slots`) _output_get_3 (make `/Game/Inventory2/Blueprints/Structures/InventorySlot` (`local.LocalClass`) 1))
        (`self.UpdateSlotAtIndex` (`local.FoundIndex`))
        (if (> (`local.LocalQuantity`) 1)
          (bind (_success_6 _rest_3) (`self.AddItem` (`local.LocalClass`) (- (`local.LocalQuantity`) 1)))
          (return true _rest_3)
          (else
            (return true 0)))
        (else
          (return false (`local.LocalQuantity`)))))))

(fn `AddItemToIndex`
  (params (Index :type Integer) (ItemClass :type "/Game/Inventory2/Blueprints/ItemClasses/ItemBP Class Reference") (Amount :type Integer))
  (returns (Success :type Boolean))
  (bind _empty_ (`self.IsSlotEmpty?` Index))
  (if (and _empty_ (<= Amount (`self.MaxStack`)))
    (`KismetArrayLibrary.Array_Set` (`self.Slots`) Index (make `/Game/Inventory2/Blueprints/Structures/InventorySlot` ItemClass Amount))
    (`self.UpdateSlotAtIndex` Index)
    (return true)
    (else
      (return false))))

(fn `AddToIndex`
  (params (FromIndex :type Integer) (ToIndex :type Integer))
  (returns (Success :type Boolean))
  (locals (LocalFrom :type Integer) (LocalTo :type Integer) (LocalClass :type "/Game/Inventory2/Blueprints/ItemClasses/ItemBP Class Reference"))
  (bind (_itemclass _quantity) (break `/Game/Inventory2/Blueprints/Structures/InventorySlot` (`|GetArrayItem` (`self.Slots`) (`local.LocalTo`))))
  (bind _itemclass_2 (break `/Game/Inventory2/Blueprints/Structures/InventorySlot` (`|GetArrayItem` (`self.Slots`) (`local.LocalFrom`))))
  (set `local.LocalFrom` FromIndex)
  (set `local.LocalTo` ToIndex)
  (bind (_empty_ _iteminfo) (`self.GetItemInfoAtIndex` (`local.LocalFrom`)))
  (if (and (`.Stackable_19_F0362273495ED642AAD4648101CE2EDC` (break `/Game/Inventory2/Blueprints/Structures/ItemInfo` _iteminfo)) (< _quantity (`self.MaxStack`)) (== _itemclass_2 _itemclass))
    (set `local.LocalClass` _itemclass_2)
    (bind _quantity_2 (`self.GetAmountAtIndex` (`local.LocalTo`)))
    (bind _quantity_3 (`self.GetAmountAtIndex` (`local.LocalFrom`)))
    (if (>= (- (`self.MaxStack`) _quantity_2) _quantity_3)
      (bind _quantity_4 (`self.GetAmountAtIndex` (`local.LocalFrom`)))
      (bind _quantity_5 (`self.GetAmountAtIndex` (`local.LocalFrom`)))
      (`KismetArrayLibrary.Array_Set` (`self.Slots`) (`local.LocalTo`) (make `/Game/Inventory2/Blueprints/Structures/InventorySlot` (`local.LocalClass`) (+ _quantity_4 _quantity_5)))
      (`KismetArrayLibrary.Array_Set` (`self.Slots`) (`local.LocalFrom`) (make `/Game/Inventory2/Blueprints/Structures/InventorySlot` null))
      (else
        (bind _quantity_6 (`self.GetAmountAtIndex` (`local.LocalFrom`)))
        (bind _quantity_7 (`self.GetAmountAtIndex` (`local.LocalTo`)))
        (`KismetArrayLibrary.Array_Set` (`self.Slots`) (`local.LocalFrom`) (make `/Game/Inventory2/Blueprints/Structures/InventorySlot` (`local.LocalClass`) (- _quantity_6 (- (`self.MaxStack`) _quantity_7))))
        (`KismetArrayLibrary.Array_Set` (`self.Slots`) (`local.LocalTo`) (make `/Game/Inventory2/Blueprints/Structures/InventorySlot` (`local.LocalClass`) (`self.MaxStack`)))))
    (`self.UpdateSlotAtIndex` (`local.LocalFrom`))
    (`self.UpdateSlotAtIndex` (`local.LocalTo`))
    (return true)
    (else
      (return false))))

(fn `GetAmountAtIndex`
  (params (Index :type Integer))
  (returns (Quantity :type Integer))
  (return (`.Quantity_5_98A095BD43ACF0309D55108942BDFC60` (break `/Game/Inventory2/Blueprints/Structures/InventorySlot` (`|GetArrayItem` (`self.Slots`) Index)))))

(fn `GetItemInfoAtIndex`
  (params (Index :type Integer))
  (returns (`Empty?` :type Boolean) (ItemInfo :type "/Game/Inventory2/Blueprints/Structures/ItemInfo Structure") (ItemQuantity :type Integer))
  (bind (_itemclass _quantity) (break `/Game/Inventory2/Blueprints/Structures/InventorySlot` (`|GetArrayItem` (`self.Slots`) Index)))
  (if (`KismetSystemLibrary.IsValidClass` _itemclass)
    (return false (defaults `Object` _itemclass) _quantity)
    (else
      (return true (struct) 0))))

(fn `HideIncinerator`
  (bind _returnvalue (`GameplayStatics.GetPlayerController` 0))
  (`Widget.SetVisibility` (`self.Incinerator Widget 0`) "Hidden")
  (set `/Game/Inventory2/Blueprints/InventoryBP.IncineratorOpen?` false (`/Game/FirstPersonBP/Blueprints/FirstPersonCharacter.InventoryRef` (`self.FirstPersonCharacter`)))
  (`WidgetBlueprintLibrary.SetInputMode_GameOnly` _returnvalue)
  (set `PlayerController.bShowMouseCursor` false _returnvalue)
  (return))

(fn `IncreaseAmountAtIndex`
  (params (Index :type Integer) (Amount :type Integer))
  (returns (Success :type Boolean))
  (bind _slots (`self.Slots`))
  (bind (_output_itemclass _output_quantity) (break `/Game/Inventory2/Blueprints/Structures/InventorySlot` (`|GetArrayItem` _slots Index)))
  (bind _empty_ (`self.IsSlotEmpty?` Index))
  (bind _quantity (`self.GetAmountAtIndex` Amount))
  (if (and (not _empty_) (<= (+ _quantity Amount) (`self.MaxStack`)))
    (`KismetArrayLibrary.Array_Set` _slots Index (make `/Game/Inventory2/Blueprints/Structures/InventorySlot` _output_itemclass (+ _output_quantity Amount)))
    (return true)
    (else
      (return false))))

(fn `InventoryToMachine`
  (params (Inventory :type "/Game/Inventory2/Blueprints/InventoryBP Object Reference") (InventoryIndex :type Integer) (IncineratorIndex :type Integer))
  (returns (Success :type Boolean))
  (locals (LocalInventory :type "/Game/Inventory2/Blueprints/InventoryBP Object Reference") (LocalInventoyIndex :type Integer) (LocalIncineratorIndex :type Integer) (AmountToAdd :type Integer :default 0))
  (bind _localinventory (`local.LocalInventory`))
  (bind _output_itemclass (break `/Game/Inventory2/Blueprints/Structures/InventorySlot` (`|GetArrayItem` (`self.Slots`) (`local.LocalIncineratorIndex`))))
  (bind _output_itemclass_2 (break `/Game/Inventory2/Blueprints/Structures/InventorySlot` (`|GetArrayItem` (`/Game/Inventory2/Blueprints/InventoryBP.Slots` _localinventory) (`local.LocalInventoyIndex`))))
  (bind _output_itemclass_3 (break `/Game/Inventory2/Blueprints/Structures/InventorySlot` (`|GetArrayItem` (`/Game/Inventory2/Blueprints/InventoryBP.Slots` (`local.LocalInventory`)) (`local.LocalInventoyIndex`))))
  (set `local.LocalInventory` Inventory)
  (set `local.LocalInventoyIndex` InventoryIndex)
  (set `local.LocalIncineratorIndex` IncineratorIndex)
  (bind _empty_ (`self.IsSlotEmpty?` (`local.LocalIncineratorIndex`)))
  (if _empty_
    (bind _quantity (`/Game/Inventory2/Blueprints/InventoryBP.GetAmountAtIndex` _localinventory (`local.LocalInventoyIndex`)))
    (set `local.AmountToAdd` _quantity)
    (bind _success (`self.AddItemToIndex` (`local.LocalIncineratorIndex`) _output_itemclass_2 (`local.AmountToAdd`)))
    (if _success
      (`/Game/Inventory2/Blueprints/InventoryBP.RemoveItemAtIndex` (`local.LocalInventory`) (`local.LocalInventoyIndex`) (`local.AmountToAdd`))
      (return true)
      (else
        (return false)))
    (else
      (bind (_empty__2 _iteminfo) (`self.GetItemInfoAtIndex` (`local.LocalIncineratorIndex`)))
      (bind _quantity_2 (`self.GetAmountAtIndex` (`local.LocalIncineratorIndex`)))
      (if (and (== _output_itemclass _output_itemclass_3) (`.Stackable_19_F0362273495ED642AAD4648101CE2EDC` (break `/Game/Inventory2/Blueprints/Structures/ItemInfo` _iteminfo)) (< _quantity_2 (`self.MaxStack`)))
        (bind _quantity_3 (`self.GetAmountAtIndex` (`local.LocalIncineratorIndex`)))
        (bind _quantity_4 (`/Game/Inventory2/Blueprints/InventoryBP.GetAmountAtIndex` (`local.LocalInventory`) (`local.LocalInventoyIndex`)))
        (bind _returnvalue (- (`self.MaxStack`) _quantity_3))
        (set `local.AmountToAdd` (`KismetMathLibrary.SelectInt` _returnvalue _quantity_4 (> _quantity_4 _returnvalue)))
        (bind _success_2 (`self.IncreaseAmountAtIndex` (`local.LocalIncineratorIndex`) (`local.AmountToAdd`)))
        (if _success_2
          (`/Game/Inventory2/Blueprints/InventoryBP.RemoveItemAtIndex` (`local.LocalInventory`) (`local.LocalInventoyIndex`) (`local.AmountToAdd`))
          (return true)
          (else
            (return false)))
        (else
          (return false))))))

(fn `IsSlotEmpty?`
  (params (Index :type Integer))
  (returns (`Empty?` :type Boolean))
  (return (not (`KismetSystemLibrary.IsValidClass` (`.ItemClass_2_105CC4C045ECF93B9A0E459DE653DFA4` (break `/Game/Inventory2/Blueprints/Structures/InventorySlot` (`|GetArrayItem` (`self.Slots`) Index)))))))

(fn `RemoveItemAtIndex`
  (params (Index :type Integer) (Quantity :type Integer))
  (returns (Success :type Boolean))
  (locals (LocalIndex :type Integer) (LocalQuantity :type Integer))
  (bind _slots (`self.Slots`))
  (bind _localindex (`local.LocalIndex`))
  (bind (_itemclass _quantity) (break `/Game/Inventory2/Blueprints/Structures/InventorySlot` (`|GetArrayItem` _slots _localindex)))
  (set `local.LocalIndex` Index)
  (set `local.LocalQuantity` Quantity)
  (bind _empty_ (`self.IsSlotEmpty?` (`local.LocalIndex`)))
  (if (and (not _empty_) (> (`local.LocalQuantity`) 0))
    (bind _quantity_2 (`self.GetAmountAtIndex` (`local.LocalIndex`)))
    (if (>= (`local.LocalQuantity`) _quantity_2)
      (`KismetArrayLibrary.Array_Set` (`self.Slots`) (`local.LocalIndex`) (make `/Game/Inventory2/Blueprints/Structures/InventorySlot` null))
      (`self.UpdateSlotAtIndex` (`local.LocalIndex`))
      (return true)
      (else
        (`KismetArrayLibrary.Array_Set` _slots _localindex (make `/Game/Inventory2/Blueprints/Structures/InventorySlot` _itemclass (- _quantity (`local.LocalQuantity`))))
        (`self.UpdateSlotAtIndex` (`local.LocalIndex`))
        (return true)))
    (else
      (return false))))

(fn `SearchAvailStack`
  (params (ItemClass :type "/Game/Inventory2/Blueprints/ItemClasses/ItemBP Class Reference"))
  (returns (Success :type Boolean) (Index :type Integer))
  (locals (LocalBool :type Boolean) (LocalIndex :type Integer))
  (for (_array_element _array_index) (`self.Slots`)
    (bind (_itemclass _quantity) (break `/Game/Inventory2/Blueprints/Structures/InventorySlot` _array_element))
    (if (`KismetSystemLibrary.IsValidClass` _itemclass)
      (if (and (== _itemclass ItemClass) (< _quantity (`self.MaxStack`)))
        (set `local.LocalBool` true)
        (set `local.LocalIndex` _array_index)
        (break))))
  (return (`local.LocalBool`) (`local.LocalIndex`)))

(fn `SearchEmptySlot`
  (returns (Success :type Boolean) (Index :type Integer))
  (locals (LocalBool :type Boolean) (LocalIndex :type Integer))
  (for (_array_element _array_index) (`self.Slots`)
    (if (not (`KismetSystemLibrary.IsValidClass` (`.ItemClass_2_105CC4C045ECF93B9A0E459DE653DFA4` (break `/Game/Inventory2/Blueprints/Structures/InventorySlot` _array_element))))
      (set `local.LocalBool` true)
      (set `local.LocalIndex` _array_index)
      (break)))
  (return (`local.LocalBool`) (`local.LocalIndex`)))

(fn `ShowIncinerator`
  (bind _returnvalue (`GameplayStatics.GetPlayerController` 0))
  (`Widget.SetVisibility` (`self.Incinerator Widget 0`) "Visible")
  (set `/Game/Inventory2/Blueprints/InventoryBP.IncineratorOpen?` true (`/Game/FirstPersonBP/Blueprints/FirstPersonCharacter.InventoryRef` (`self.FirstPersonCharacter`)))
  (`WidgetBlueprintLibrary.SetInputMode_GameAndUIEx` _returnvalue (`self.MainWidget`))
  (set `PlayerController.bShowMouseCursor` true _returnvalue)
  (return))

(fn `SplitStackToIndex`
  (params (FromIndex :type Integer) (ToIndex :type Integer) (Quantity :type Integer))
  (returns (Success :type Boolean))
  (locals (LocalFrom :type Integer) (LocalTo :type Integer) (LocalQuantity :type Integer) (LocalClass :type "/Game/Inventory2/Blueprints/ItemClasses/ItemBP Class Reference"))
  (bind (_itemclass _quantity) (break `/Game/Inventory2/Blueprints/Structures/InventorySlot` (`|GetArrayItem` (`self.Slots`) (`local.LocalFrom`))))
  (set `local.LocalFrom` FromIndex)
  (set `local.LocalTo` ToIndex)
  (set `local.LocalQuantity` Quantity)
  (bind _empty_ (`self.IsSlotEmpty?` (`local.LocalTo`)))
  (bind _empty__2 (`self.IsSlotEmpty?` (`local.LocalFrom`)))
  (bind (_empty__3 _iteminfo _itemquantity) (`self.GetItemInfoAtIndex` (`local.LocalFrom`)))
  (if (and _empty_ (not _empty__2) (`.Stackable_19_F0362273495ED642AAD4648101CE2EDC` (break `/Game/Inventory2/Blueprints/Structures/ItemInfo` _iteminfo)) (> _itemquantity 1) (> _itemquantity (`local.LocalQuantity`)))
    (bind _output_get (set `local.LocalClass` _itemclass))
    (`KismetArrayLibrary.Array_Set` (`self.Slots`) (`local.LocalFrom`) (make `/Game/Inventory2/Blueprints/Structures/InventorySlot` _output_get (- _quantity (`local.LocalQuantity`))))
    (`KismetArrayLibrary.Array_Set` (`self.Slots`) (`local.LocalTo`) (make `/Game/Inventory2/Blueprints/Structures/InventorySlot` (`local.LocalClass`) (`local.LocalQuantity`)))
    (`self.UpdateSlotAtIndex` (`local.LocalFrom`))
    (`self.UpdateSlotAtIndex` (`local.LocalTo`))
    (return true)
    (else
      (return false))))

(fn `SwapSlots`
  (params (Index1 :type Integer) (Index2 :type Integer))
  (returns (Success :type Boolean))
  (locals (LocalIndex1 :type Integer) (LocalIndex2 :type Integer) (LocalSlot2 :type "/Game/Inventory2/Blueprints/Structures/InventorySlot Structure"))
  (set `local.LocalIndex1` Index1)
  (set `local.LocalIndex2` Index2)
  (if (or (> (`local.LocalIndex1`) (`KismetArrayLibrary.Array_LastIndex` (`self.Slots`))) (> (`local.LocalIndex2`) (`KismetArrayLibrary.Array_LastIndex` (`self.Slots`))))
    (return false)
    (else
      (set `local.LocalSlot2` (`|GetArrayItem` (`self.Slots`) (`local.LocalIndex2`)))
      (`KismetArrayLibrary.Array_Set` (`self.Slots`) (`local.LocalIndex2`) (`|GetArrayItem` (`self.Slots`) (`local.LocalIndex1`)))
      (`KismetArrayLibrary.Array_Set` (`self.Slots`) (`local.LocalIndex1`) (`local.LocalSlot2`))
      (`self.UpdateSlotAtIndex` (`local.LocalIndex1`))
      (`self.UpdateSlotAtIndex` (`local.LocalIndex2`))
      (return true))))

(fn `UserConstructionScript`)